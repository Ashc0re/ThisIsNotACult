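; FL_UI is a function library of cultist and building-action helpers, named for UI use.
; It flattens cultist maps into arrays, checks availability, removes map entries matching a given availability, and looks up a building's current actions.
; Setters rebuild each cultist struct and write it back through game mode messages to update availability or action text.
; The action-text setter looks cultists up by array index, unlike the availability setter, which uses ID.
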(fn `AreCultistsAvailable?`
  (params (CultistsToCheck :type "Map of Integer to /Game/Blueprints/Utlility/Struct_Cultist Structure"))
  (returns (ReturnValue :type Boolean))
  (bind (_keypin _valuepin) (`|MapForEach` CultistsToCheck)
    (:`then`
      (bind (_id _name _isplayer_ _body _mind _idling _availability) (break `/Game/Blueprints/Utlility/Struct_Cultist` _valuepin))
      (if (not (or (`|EnumEquality` _availability "NewEnumerator0") (`|EnumEquality` _availability "NewEnumerator4")))
        (return false)))
    (:`CompletedPin`
      (return true))))

(fn `CultistMapIntoArray`
  (params (Map :type "Map of Integer to /Game/Blueprints/Utlility/Struct_Cultist Structure (by ref)"))
  (returns (Array :type "Array of /Game/Blueprints/Utlility/Struct_Cultist Structure"))
  (locals (_Array :type "Array of /Game/Blueprints/Utlility/Struct_Cultist Structure"))
  (bind (_keypin _valuepin) (`|MapForEach` Map)
    (:`then`
      (`KismetArrayLibrary.Array_Add` (`local._Array`) _valuepin))
    (:`CompletedPin`
      (return (`local._Array`)))))

(fn `GetCultistsOfAvailability(Map)`
  (params (Map :type "Map of Integer to /Game/Blueprints/Utlility/Struct_Cultist Structure (by ref)") (Availability :type "/Game/Blueprints/Utlility/Enum_CultistAvailability Enum" :default "NewEnumerator0"))
  (returns (ReturnValue :type "Map of Integer to /Game/Blueprints/Utlility/Struct_Cultist Structure (by ref)"))
  (locals (_Output :type "Map of Integer to /Game/Blueprints/Utlility/Struct_Cultist Structure"))
  (bind (_keypin _valuepin) (`|MapForEach` Map)
    (:`then`
      (if (not (`|EnumInequality` (`local.Availability`) (`.Availability_30_50F075E3439C9F7901F7D4ADEE0D3873` (break `/Game/Blueprints/Utlility/Struct_Cultist` _valuepin))))
        (`BlueprintMapLibrary.Map_Remove` (`local.Map`) _keypin)))
    (:`CompletedPin`
      (return (`local.Map`)))))

(fn `IsActionActive?`
  (params (Building :type "/Game/Blueprints/Buildings/_BP_Building_Base Object Reference") (ActionIndex :type "Integer (by ref)"))
  (returns (ReturnValue :type Boolean))
  (return (`.ReturnValue` (`BlueprintMapLibrary.Map_Find` (`/Game/Blueprints/Buildings/_BP_Building_Base.CurrentActions` Building) ActionIndex))))

(fn `SetCultistActionString`
  (params (Action :type String) (Cultists :type "Array of /Game/Blueprints/Utlility/Struct_Cultist Structure") (Building :type String) (Idling :type Boolean))
  (if Idling
    (for (_array_element _array_index) Cultists
      (bind (_cultistfound _cultist _cultistindex) (message `/Game/Blueprints/Utlility/BPI_GameMode.FindCultistByID` (`GameplayStatics.GetGameMode` null) _array_index))
      (if _cultistfound
        (bind (_id _name _isplayer_ _body _mind _idling) (break `/Game/Blueprints/Utlility/Struct_Cultist` _array_element))
        (message `/Game/Blueprints/Utlility/BPI_GameMode.UpdateCultist` (`GameplayStatics.GetGameMode` null) _cultistindex (make `/Game/Blueprints/Utlility/Struct_Cultist` _id _name _isplayer_ _body _mind _idling "NewEnumerator0" "Idling"))))
    (else
      (for (_array_element_2 _array_index_2) Cultists
        (bind (_cultistfound_2 _cultist_2 _cultistindex_2) (message `/Game/Blueprints/Utlility/BPI_GameMode.FindCultistByID` (`GameplayStatics.GetGameMode` null) _array_index_2))
        (if _cultistfound_2
          (bind (_id_2 _name_2 _isplayer__2 _body_2 _mind_2 _idling_2) (break `/Game/Blueprints/Utlility/Struct_Cultist` _array_element_2))
          (message `/Game/Blueprints/Utlility/BPI_GameMode.UpdateCultist` (`GameplayStatics.GetGameMode` null) _cultistindex_2 (make `/Game/Blueprints/Utlility/Struct_Cultist` _id_2 _name_2 _isplayer__2 _body_2 _mind_2 _idling_2 "NewEnumerator0" (`KismetStringLibrary.Concat_StrStr` "Is " (`local.Action`) " at " (`local.Building`)))))))))

(fn `SetCultistAvailability(Map)`
  (params (Map :type "Map of Integer to /Game/Blueprints/Utlility/Struct_Cultist Structure (by ref)") (Availability :type "/Game/Blueprints/Utlility/Enum_CultistAvailability Enum" :default "NewEnumerator0"))
  (locals (_GameMode :type "/Game/Blueprints/GameMode/GM_Cult Object Reference"))
  (bind _array (`self.CultistMapIntoArray` Map))
  (`self.SetCultsitAvailability(Array)` _array (`local.Availability`)))

(fn `SetCultsitAvailability(Array)`
  (params (CultistsToUpdate :type "Array of /Game/Blueprints/Utlility/Struct_Cultist Structure (by ref)") (Availability :type "/Game/Blueprints/Utlility/Enum_CultistAvailability Enum" :default "NewEnumerator0"))
  (for _array_element CultistsToUpdate
    (bind (_id _name _isplayer_ _body _mind _idling _availability _actionmessage) (break `/Game/Blueprints/Utlility/Struct_Cultist` _array_element))
    (bind (_cultistfound _cultist _cultistindex) (message `/Game/Blueprints/Utlility/BPI_GameMode.FindCultistByID` (`GameplayStatics.GetGameMode` null) _id))
    (message `/Game/Blueprints/Utlility/BPI_GameMode.UpdateCultist` (`GameplayStatics.GetGameMode` null) _cultistindex (make `/Game/Blueprints/Utlility/Struct_Cultist` _id _name _isplayer_ _body _mind _idling Availability _actionmessage))))