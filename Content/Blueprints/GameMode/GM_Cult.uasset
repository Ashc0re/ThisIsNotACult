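; GM_Cult is the game mode for a cult management game, owning the clock, coins, Insight and the cultist roster.
; A looping timeline counts minutes and passes hours, progressing every BPI_Buildings actor, with noon upkeep and escalating debt that triggers a game-over popup.
; Recruitment adds the player or randomly named, unique-ID cultists.
; RequestAction checks action and cultist availability before handing work to a building; FindCultistByID is a stub.
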(event `self.ReceiveBeginPlay`
  ; Initialize Game
  ;; Get reference to Player Actor
  (bind _asbp_player (cast `/Game/Blueprints/Player/BP_Player` (`GameplayStatics.GetPlayerCharacter` 0)))
  (set `self.PlayerActor` _asbp_player)
  ;; Start DayTime Cycle
  (`self.Event_ResetDayTimeCycle`)
  ;; Wait For UI
  (`KismetSystemLibrary.Delay` 0.2)
  ;; Add Player Cultist
  (`self.RecruitCultist` (`self.Player Name`) true 1 1))

(event `Event_ResetDayTimeCycle`
  ; DayTimeCycle Handler
  (bind (_direction _minutespassing) (`Timeline|TL_DayTime` :!via `PlayFromStart` :!label _label)
    (:`Update`
      (set `self.Minutes` _minutespassing))
    (:`Finished`
      (`self.PassHour`))))

(event `Event_UnpauseDayTimeCycle`
  ; DayTimeCycle Handler
  (goto _label))

(event `Event_PauseDayTimeCylce`
  ; DayTimeCycle Handler
  (goto _label :!via `Stop`))

(event `/Game/Blueprints/Utlility/BPI_GameMode.AddCoins`
  (params (CoinsToAdd :type Integer))
  ; Coins
  (set `self.Coins` (+ CoinsToAdd (`self.Coins`))))

(event `/Game/Blueprints/Utlility/BPI_GameMode.DeductCoins`
  (params (_CoinsToDeduct :type Integer))
  ; Coins
  (set `self.Coins` (- (`self.Coins`) _CoinsToDeduct)))

(event `/Game/Blueprints/Utlility/BPI_GameMode.GameOver`
  (`DestroySessionCallbackProxy.DestroySession` (`GameplayStatics.GetPlayerController` 0)))

(event `/Game/Blueprints/Utlility/BPI_GameMode.AddInsight`
  (params (Amount :type Integer))
  ; Insight
  (set `self.Insight` (+ Amount (`self.Insight`))))

(event `/Game/Blueprints/Utlility/BPI_GameMode.DeductInsight`
  (params (Amount :type Integer))
  ; Insight
  (set `self.Insight` (- (`self.Insight`) Amount)))

(event `/Game/Blueprints/Utlility/BPI_GameMode.UpdateCultist`
  (params (Index :type Integer) (Cultist :type "/Game/Blueprints/Utlility/Structs/Struct_Cultist Structure"))
  (`KismetArrayLibrary.Array_Set` (`self.Recruited Cultists`) Index Cultist))

(fn `DebtCheck`
  (if (< (`self.Coins`) 0)
    (bind _result (`/Engine/EditorBlueprintResources/StandardMacros.IncrementInt` (`self.DebtLevel`))
      (:`  `
        (if (== _result 3)
          (bind _asbp_player_controller (cast `/Game/Blueprints/Player/BP_PlayerController` (`GameplayStatics.GetPlayerController` 0)))
          (`/Game/Blueprints/Player/BP_PlayerController.Event_CreatePopup` _asbp_player_controller "/Game/Blueprints/UI/Menus/PopUps/WBP_Popup_GameOver.WBP_Popup_GameOver_C")
          (return))))
    (else
      (if (> (`self.DebtLevel`) 0)
        (`/Engine/EditorBlueprintResources/StandardMacros.DecrementInt` (`self.DebtLevel`)
          (:`  `
            _)))
      (return))))

(fn `Debug_PrintCultistOverview`
  (`KismetSystemLibrary.PrintString` (`KismetStringLibrary.Concat_StrStr` "Curent Cultists: " (`KismetStringLibrary.Conv_IntToString` (`KismetArrayLibrary.Array_Length` (`self.Recruited Cultists`)))) true true (struct :`G` 0.66 :`B` 1.0 :`A` 1.0) 10.0)
  (for _array_element (`self.Recruited Cultists`)
    (bind (_id _name _isplayer_ _body _mind) (break `/Game/Blueprints/Utlility/Structs/Struct_Cultist` _array_element))
    (`KismetSystemLibrary.PrintString` (`KismetStringLibrary.Concat_StrStr` "ID: " (`KismetStringLibrary.Conv_IntToString` _id) " | Name: " _name " | IsPlayer?: " (`KismetStringLibrary.Conv_BoolToString` _isplayer_) " | Body: " (`KismetStringLibrary.Conv_IntToString` _body) " | Mind:" (`KismetStringLibrary.Conv_IntToString` _mind)) true true (struct :`G` 0.66 :`B` 1.0 :`A` 1.0) 10.0)))

(fn `FindCultistByID`
  (params (ID :type Integer))
  (returns (CultistFound :type Boolean) (Cultist :type "/Game/Blueprints/Utlility/Structs/Struct_Cultist Structure") (CultistIndex :type Integer))
  (return false (struct) 0))

(fn `GenerateUniqueCultistID`
  (returns (NewID :type Integer))
  (locals (_NewID :type Integer :default 0) (`_IsIDReserved?` :type Boolean))
  (for _ (range 1 1000)
    (set `local._NewID` (`KismetMathLibrary.RandomIntegerInRange` 1 999))
    (set `local._IsIDReserved?` false)
    (for _array_element (`self.Recruited Cultists`)
      (if (== (`.ID_11_EAAB6FCC40377C673E6074AE23299FB3` (break `/Game/Blueprints/Utlility/Structs/Struct_Cultist` _array_element)) (`local._NewID`))
        (set `local._IsIDReserved?` true)))
    (if (not (`local._IsIDReserved?`))
      (return (`local._NewID`))))
  (`KismetSystemLibrary.RaiseScriptError` "No valid Cultist ID could be generated.")
  (return (+ (`local._NewID`) 1000)))

(fn `GetCoins`
  (returns (Coins :type Integer))
  (return (`self.Coins`)))

(fn `GetCurrentCultists`
  (returns (CurrentCultists :type "Array of /Game/Blueprints/Utlility/Structs/Struct_Cultist Structure"))
  (return (`self.Recruited Cultists`)))

(fn `GetCurrentDay`
  (returns (Day :type Integer))
  (return (`self.Day`)))

(fn `GetCurrentHour`
  (returns (CurrentHour :type Integer))
  (return (`self.Hour`)))

(fn `GetCurrentMinute`
  (returns (CurrentMinute :type "Float (double-precision)"))
  (return (`self.Minutes`)))

(fn `GetInsight`
  (returns (Insight :type Integer))
  (return (`self.Insight`)))

(fn `GetRandomCultistName`
  (returns (Name :type String))
  (locals (_Key :type String))
  (bind _output_get (set `local._Key` (`KismetStringLibrary.Conv_IntToString` (`KismetMathLibrary.RandomIntegerInRange` 1 10))))
  (switch `int` (`KismetStringLibrary.Len` _output_get)
    (:`1`
      (set `local._Key` (`KismetStringLibrary.Concat_StrStr` "00" (`local._Key`))))
    (:`2`
      (set `local._Key` (`KismetStringLibrary.Concat_StrStr` "0" (`local._Key`)))))
  (bind _returnvalue (`|GetDataTableRow` "/Game/Blueprints/Utlility/DT_CultistNames.DT_CultistNames" (`KismetStringLibrary.Conv_StringToName` (`local._Key`)))
    (:`then`
      (return (`.Name_2_BEAF6EBA46DEF2922E365AAABA40037D` (break `/Game/Blueprints/Utlility/Structs/Struct_CultistName` _returnvalue))))))

(fn `PassDay`
  (set `self.Hour` 0)
  (`/Engine/EditorBlueprintResources/StandardMacros.IncrementInt` (`self.Day`)))

(fn `PassHour`
  ; Check if a new day should start
  (if (== (`self.Hour`) (- (`self.DayLength`) 1))
    (`self.PassDay`)
    (else
      (`/Engine/EditorBlueprintResources/StandardMacros.IncrementInt` (`self.Hour`)
        (:`  `
          _))))
  ; Progress work each passing hour at every building
  (bind _outactors (`GameplayStatics.GetAllActorsWithInterface` "/Game/Blueprints/Utlility/BPI_Buildings.BPI_Buildings_C"))
  (for _array_element _outactors
    (message `/Game/Blueprints/Utlility/BPI_Buildings.ProgressAction` _array_element))
  ; At noon, deduct Upkeep from players coins
  (if (== (`self.Hour`) (/ (`self.DayLength`) 2))
    (`/Game/Blueprints/Utlility/BPI_GameMode.DeductCoins` (`self.Upkeep`))
    (`self.DebtCheck`)
    (`self.Event_ResetDayTimeCycle`)
    (else
      (`self.Event_ResetDayTimeCycle`))))

(fn `RecruitCultist`
  (params (Name :type String) (IsPlayer :type Boolean) (Body :type Integer) (Mind :type Integer))
  (returns (ReturnValue :type Integer))
  (locals (_NewCultist :type "/Game/Blueprints/Utlility/Structs/Struct_Cultist Structure") (_ID :type Integer :default 0))
  (set `local._NewCultist` (make `/Game/Blueprints/Utlility/Structs/Struct_Cultist` 0 Name IsPlayer Body Mind true "NewEnumerator0" "Idling"))
  (if IsPlayer
    (`KismetArrayLibrary.Array_Add` (`self.Recruited Cultists`) (`local._NewCultist`))
    (bind _slotwidget (message `/Game/Blueprints/Utlility/BPI_Player.GetMenuSlot` (`GameplayStatics.GetPlayerController` 0) "NewEnumerator4" :!label _label))
    (message `/Game/Blueprints/Utlility/BPI_UI.UpdateWidget` (`PanelWidget.GetChildAt` _slotwidget 0))
    (return (`local._ID`))
    (elif true
      (bind _newid (`self.GenerateUniqueCultistID`))
      (bind _output_get (set `local._ID` _newid))
      (`KismetArrayLibrary.Array_Add` (`self.Recruited Cultists`) (make `/Game/Blueprints/Utlility/Structs/Struct_Cultist` _output_get (`self.GetRandomCultistName`) false (`local.Body`) (`local.Mind`) true "NewEnumerator0" "Idling"))
      (goto _label))))

(fn `RequestAction`
  (params (Cultists :type "Map of Integer to /Game/Blueprints/Utlility/Structs/Struct_Cultist Structure") (Building :type "/Game/Blueprints/Buildings/_BP_Building_Base Object Reference") (ActionIndex :type Integer))
  (returns (ActionStarted :type Boolean))
  (bind (_name _requiredtime _eventoutcome _generatesheat) (break `/Game/Blueprints/Utlility/Structs/Struct_ActionDefinition` (`BlueprintMapLibrary.Map_Find` (`/Game/Blueprints/Buildings/_BP_Building_Base.ActionDefinition` (`local.Building`)) (`local.ActionIndex`))))
  (if (and (not (`/Game/Blueprints/Utlility/FunctionLibraries/FL_Cultists.IsActionActive?` Building ActionIndex)) (`/Game/Blueprints/Utlility/FunctionLibraries/FL_Cultists.AreCultistsAvailable?` Cultists))
    (`/Game/Blueprints/Utlility/FunctionLibraries/FL_Cultists.SetCultistAvailability(Map)` :`Availability` "NewEnumerator5")
    (message `/Game/Blueprints/Utlility/BPI_Buildings.AddAction` (`local.Building`) (make `/Game/Blueprints/Utlility/Structs/Struct_ActionInstance` _name 0 _requiredtime (`local.Cultists`) _generatesheat _eventoutcome) (`local.ActionIndex`))
    (return true)
    (else
      (return false))))

(fn `UserConstructionScript`)